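; Player controller for a multiplayer match that handles character spawning, player displays, UI messages and the victory sequence.
; It spawns and possesses a MyCharacterBP at a random location, and in the Game level places a named Zhanlan display with spotlight by player number.
; Other events relay start, loading, kill and winner messages to UI2 and toggle pawn input.
; On victory it plays the winner's animation, blends the camera there, then destroys the session.
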(event Custom|UIAddWinner
  (bind _ui2 (Variables|Default|GetUI2))
  (Utilities|IsValid _ui2
    (:Is%20Valid
      (Default|AddWinner _ui2))))

(event Custom|MulticastPlaySound
  (params (Sound :type Sound%20Base%20Object%20Reference))
  (Audio|PlaySound2D Sound))

(event EventBeginPlay
  (bind _returnvalue (Game|GetPlayerCharacter 0))
  (Utilities|IsValid (Variables|Default|GetControllerPawn) :!label _label
    (:Is%20Not%20Valid
      (Utilities|IsValid _returnvalue
        (:Is%20Valid
          (Variables|Default|SetControllerPawn _returnvalue))
        (:Is%20Not%20Valid
          _))
      (Utilities|FlowControl|Delay 0.2)
      (goto _label))))

(event EventTick
  (params (DeltaSeconds :type Float%20%28single-precision%29)))

(event EventAddStartMessage
  (bind _ui2 (Variables|Default|GetUI2))
  (Utilities|IsValid _ui2
    (:Is%20Valid
      (Default|GameStart _ui2))))

(event EventSpawnCharacter
  (bind _returnvalue (Game|SpawnActorfromClass "/Game/myBlueprint/MyCharacterBP.MyCharacterBP_C" (Math|Transform|MakeTransform (Math|Vector|MakeVector (Math|Random|RandomFloatinRange 5e+01 5e+02) (Math|Random|RandomFloatinRange 5e+01 5e+02) 9e+02)) "AlwaysSpawn" 0 self (Variables|Default|GetController_ID)))
  (Variables|/Script/FightWithBlock.MyCharacter|SetCharacterName _returnvalue (Variables|Default|GetMyName))
  (Variables|Default|SetControllerPawn _returnvalue)
  (Pawn|Possess _returnvalue)
  (Utilities|FlowControl|Delay 0.2)
  (Class|MyPlayerController|SetPosses))

(event EventSpawnMoxing
  (bind _playernum (Variables|Default|GetPlayerNum))
  (bind _returnvalue (- _playernum 1))
  (bind _returnvalue_2 (Utilities|Select :Index _returnvalue :Option%200 "-100.000000,100.000000,-800.000000" :Option%201 "-100.000000,300.000000,-600.000000" :Option%202 "-300.000000,300.000000,-800.000000" :Option%203 "-300.000000,500.000000,-600.000000" :Option%204 "-500.000000,500.000000,-800.000000"))
  (bind _returnvalue_3 (Game|GetCurrentLevelName true))
  (if (Utilities|Enum|Equal(Enum) _returnvalue_3 "Game")
    (Utilities|FlowControl|Delay 1.0)
    (bind _returnvalue_4 (Game|SpawnActorfromClass "/Game/myBlueprint/zhanlan.zhanlan_C" (Math|Transform|MakeTransform _returnvalue_2 "0,225.000000, 0" "1,1,1") "AdjustIfPossibleButAlwaysSpawn" 0 self _playernum))
    (Game|SpawnActorfromClass "/Game/myBlueprint/zhanlanSpotLight.zhanlanSpotLight_C" (Math|Transform|MakeTransform (+ _returnvalue_2 "0, 0,100.000000") "0,225.000000, 0" "1,1,1") "AdjustIfPossibleButAlwaysSpawn" 0 0)
    (Variables|Default|SetRzhanlan _returnvalue_4)
    (CallFunction|MulticastPlaySound "/Game/Audio/通电音01.通电音01")))

(event EventPrintKillMessage
  (params (Name :type Name))
  (bind _ui2 (Variables|Default|GetUI2))
  (Utilities|IsValid _ui2
    (:Is%20Valid
      (Default|PrintKillMessage _ui2 Name))))

(event EventEndText
  (bind _ui2 (Variables|Default|GetUI2))
  (Utilities|IsValid _ui2
    (:Is%20Valid
      (Default|RemoveText _ui2))))

(event EventControllerReady
  (bind _ui2 (Variables|Default|GetUI2))
  (Utilities|IsValid _ui2
    (:Is%20Valid
      (Default|RemoveStart _ui2)
      (Utilities|FlowControl|Delay 0.2)
      (Default|AddText _ui2 "地图生成中"))))

(event EventTargetMovetoWinner
  (params (Controller :type My%20Player%20Controller%20Object%20Reference))
  (bind _returnvalue (Game|GetGameInstance))
  (bind _returnvalue_2 (Pawn|GetControlledPawn Controller))
  (Utilities|IsValid Controller
    (:Is%20Valid
      (Utilities|IsValid _returnvalue_2
        (:Is%20Valid
          (bind _asmy_character_bp (Utilities|Casting|CastToMyCharacterBP _returnvalue_2))
          (Default|PlayVictorAnim _asmy_character_bp)
          (Game|Player|SetViewTargetwithBlend _returnvalue_2 1.5 "VTBlend_Linear" 0.0 false)
          (CallFunction|UIAddWinner)
          (Utilities|FlowControl|Delay 7.0)
          (Utilities|IsValid _returnvalue
            (:Is%20Valid
              (bind _asbpmy_game_instance (Utilities|Casting|CastToBPMyGameInstance _returnvalue))
              (Default|DestroySession _asbpmy_game_instance))))))))

(event EventSetzhanlan
  (bind _rzhanlan (Variables|Default|GetRzhanlan))
  (Utilities|IsValid _rzhanlan
    (:Is%20Valid
      (Variables|/Game/myBlueprint/zhanlan.zhanlan_C|SetName _rzhanlan (Variables|Default|GetMyName)))))

(event EventSetAllowInput
  (params (Choose :type Boolean))
  (bind _returnvalue (Pawn|GetControlledPawn))
  (Utilities|IsValid _returnvalue
    (:Is%20Valid
      (bind _asmy_character_bp (Utilities|Casting|CastToMyCharacterBP _returnvalue))
      (Class|MyCharacter|ClientSetAllowInput _asmy_character_bp Choose))))

(fn ConstructionScript)