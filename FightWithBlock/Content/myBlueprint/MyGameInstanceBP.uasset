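; Game instance Blueprint that tracks room readiness and releases the game once every entry is ready.
; GetSelf finds the RoomInfo entry whose Owner matches the supplied GameState and rewrites it as ready.
; It then scans the array and, if all entries are ready, removes all widgets and unpauses the game.
; Debug strings trace the loop, and the Print function is an empty stub.
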(fn GetSelf
  (params (GameState :type Game%20State%20Base%20Object%20Reference))
  (bind (_array_element _array_index) (Utilities|Array|ForEachLoopwithBreak (Variables|Default|GetRoomInfo) :!label _label)
    (:LoopBody
      (Development|PrintString "Loop" true true "(R=0.000000,G=0.660000,B=1.000000,A=1.000000)" 5.0)
      (if (== GameState (.Owner (Utilities|Struct|BreakRoomInfo _array_element)))
        (Utilities|Array|SetArrayElem (Variables|Default|GetRoomInfo) _array_index (Utilities|Struct|MakeRoomInfo (.Owner (Utilities|Struct|BreakRoomInfo _array_element)) (.Name (Utilities|Struct|BreakRoomInfo _array_element)) true))
        (goto _label Break)))
    (:Completed
      (Development|PrintString "Over" true true "(R=0.000000,G=0.660000,B=1.000000,A=1.000000)" 1.2e+02)
      (bind _array_element_2 (Utilities|Array|ForEachLoopwithBreak (Variables|Default|GetRoomInfo))
        (:LoopBody
          (if (not (.IsReady (Utilities|Struct|BreakRoomInfo _array_element_2)))
            (return)))
        (:Completed
          (Viewport|RemoveAllWidgets)
          (Game|SetGamePaused false)
          (return))))))

(fn Print)