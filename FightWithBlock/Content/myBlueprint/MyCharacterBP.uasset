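; Playable hero character Blueprint that handles the presentation side: overhead life bar, HUD block slots, montages and camera shake.
; After a five-second delay, RefreshLifeBar compares camp with the local player's for friendliness and creates the life-bar widget.
; Tick billboards that widget against the player's camera and updates its health percent from HeroProperty.
; Events forward block add, remove and selection to the HUD, play pick and death montages, and toggle input; Menu input flip-flops the menu.
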(event Custom|Event_PickPlayAnim
  ;[1 1 1] Anim
  ;;[1 1 1] PickAnim
  (Animation|Montage|MontagePlay (Components|SkeletalMesh|GetAnimInstance (Variables|Character|GetMesh)) (Variables|Animation|GetAnim_Pick) 1.0 "MontageLength" 0.0))

(event Custom|Event_DeathPlayAnim
  ;[1 1 1] Anim
  ;;[1 1 1] DeadAnim
  (Animation|Montage|MontagePlay (Components|SkeletalMesh|GetAnimInstance (Variables|Character|GetMesh)) (Variables|Animation|GetAnim_Death) 1.0 "MontageLength" 0.0))

(event EventBeginPlay)

(event Collision|EventActorBeginOverlap
  (params (OtherActor :type Actor%20Object%20Reference)))

(event EventRefreshLifeBar
  (bind _mycamp (Variables|Default|GetMyCamp))
  (Utilities|FlowControl|Delay 5.0)
  (bind _asmy_character_bp (Utilities|Casting|CastToMyCharacterBP (Game|GetPlayerCharacter 0)))
  (if (Utilities|Enum|Equal(Enum) _mycamp "EDefault")
    _
    (else
      _))
  (Variables|Default|SetIsFriendy (Utilities|Enum|Equal(Enum) (Variables|/Script/FightWithBlock.MyCharacter|GetMyCamp _asmy_character_bp) _mycamp))
  (bind _returnvalue (UserInterface|CreateWidget "/Game/UMG/widgetLifeBar.widgetLifeBar_C" (Game|GetPlayerController 0) self (Variables|Default|GetHeroName)))
  (UserInterface|SetWidget (Variables|Default|GetWidget) _returnvalue))

(event EventSetAllowInput
  (params (Choose :type Boolean))
  (bind _returnvalue (Game|GetPlayerController 0))
  (if Choose
    (Input|EnableInput _returnvalue)
    (else
      (Input|DisableInput _returnvalue))))

(event EventNowChooseUI
  (params (NowChoose :type Integer))
  (bind _myhud (Variables|Default|GetmyHUD))
  (Utilities|IsValid _myhud
    (:Is%20Valid
      (Default|NowChoose (Variables|/Game/UMG/myHUD.myHUD_C|GetUI _myhud) NowChoose))))

(event EventAddBlockUI
  (params (ChooseNum :type Integer) (ChangeBlcok :type Block%20Structure))
  (bind _myhud (Variables|Default|GetmyHUD))
  (Utilities|IsValid _myhud
    (:Is%20Valid
      (Default|AddBlock (Variables|/Game/UMG/myHUD.myHUD_C|GetUI _myhud) (Variables|Default|GetNowChoose) ChooseNum (.tubiao (Utilities|Struct|BreakBlock ChangeBlcok))))
    (:Is%20Not%20Valid
      (Development|PrintString "NoUI"))))

(event EventTick
  (params (DeltaSeconds :type Float%20%28single-precision%29))
  (bind _heroproperty (Variables|Default|GetHeroProperty))
  (bind (_id _dname _pname _miaoshu _tubiao _lifevalue _maxlifevalue) (Utilities|Struct|BreakHero _heroproperty))
  (bind _asmy_character_bp (Utilities|Casting|CastToMyCharacterBP (Game|GetPlayerCharacter 0)))
  (Transformation|SetWorldRotation (Variables|Default|GetWidget) (Math|Conversions|RotationFromXVector (- "0, 0, 0" (Math|Vector|GetForwardVector (Variables|/Script/FightWithBlock.MyCharacter|GetCamera _asmy_character_bp)))) false false)
  (bind _aswidget_life_bar (Utilities|Casting|CastTowidgetLifeBar (UserInterface|GetUserWidgetObject (Variables|Default|GetWidget))))
  (Variables|/Game/UMG/widgetLifeBar.widgetLifeBar_C|SetMypercent _aswidget_life_bar (/ (Math|Conversions|ToFloat(Integer) _lifevalue) (Math|Conversions|ToFloat(Integer) _maxlifevalue))))

(event EventShakeCamera
  (Camera|PlayWorldCameraShake "/Game/myBlueprint/UnderAttackShake.UnderAttackShake_C" (Transformation|GetActorLocation) 0.0 1.5e+02 1.0))

(event EventRemoveBlockUI
  (params (ChooseNum :type Integer))
  (bind _myhud (Variables|Default|GetmyHUD))
  (Utilities|IsValid _myhud
    (:Is%20Valid
      (Default|RemoveBlock (Variables|/Game/UMG/myHUD.myHUD_C|GetUI _myhud) ChooseNum))))

(event Input|ActionEvents|InputActionMenu
  (params (Key :type Key%20Structure :default "AnyKey"))
  (bind _myhud (Variables|Default|GetmyHUD))
  (bind _ui (Variables|/Game/UMG/myHUD.myHUD_C|GetUI _myhud))
  (:Pressed
    (Utilities|IsValid _myhud
      (:Is%20Valid
        (Utilities|IsValid _ui
          (:Is%20Valid
            (Utilities|FlowControl|FlipFlop
              (:A
                (Default|OPenMenu _ui))
              (:B
                (Default|CloseMenu _ui)))))))))

(fn ConstructionScript)